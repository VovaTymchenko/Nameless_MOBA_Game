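; BP_Camera is a top-down style camera pawn that the first player controller possesses on BeginPlay, providing edge scrolling and zoom.
; Each Tick it reads the platform mouse position and shifts the actor along X or Y by Speed at screen edges, using hardcoded 1920x1080 thresholds without delta-time scaling.
; Mouse wheel presses raise or lower the actor on Z by Zoom, with no height limits.
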(event EventBeginPlay
  (Pawn|Possess (Game|GetPlayerController 0) self))

(event EventTick
  (params (DeltaSeconds :type Float%20%28single-precision%29))
  (bind _self self)
  (bind _self_2 self)
  (bind _self_3 self)
  (bind _self_4 self)
  (bind _speed (Variables|Default|GetSpeed))
  (bind _returnvalue (Transformation|GetActorLocation _self_2))
  (bind _returnvalue_2 (Transformation|GetActorLocation _self_3))
  (bind _returnvalue_3 (Transformation|GetActorLocation _self_4))
  (bind _returnvalue_4 (Transformation|GetActorLocation _self))
  (bind _returnvalue_5 (Class|WidgetLayoutLibrary|GetMousePositiononPlatform))
  (Utilities|FlowControl|Sequence
    (:then_0
      ;[0 0 0] X
      (if (< (.x _returnvalue_5) 1.0)
        (Transformation|SetActorLocation _self_3 (Math|Vector|MakeVector (+ (.x _returnvalue_2) _speed) (.y _returnvalue_2) (.z _returnvalue_2)) false false)
        (elif (> (.x _returnvalue_5) 1918.0)
          (Transformation|SetActorLocation _self_4 (Math|Vector|MakeVector (- (.x _returnvalue_3) _speed) (.y _returnvalue_3) (.z _returnvalue_3)) false false))))
    (:then_1
      ;[0 0 0] Y
      (if (< (.y _returnvalue_5) 1.0)
        (Transformation|SetActorLocation _self_2 (Math|Vector|MakeVector (.x _returnvalue) (+ (.y _returnvalue) _speed) (.z _returnvalue)) false false)
        (elif (> (.y _returnvalue_5) 1078.0)
          (Transformation|SetActorLocation _self (Math|Vector|MakeVector (.x _returnvalue_4) (- (.y _returnvalue_4) _speed) (.z _returnvalue_4)) false false))))))

(event Input|MouseEvents|MouseWheelUp
  (params (Key :type Key%20Structure :default "None"))
  (bind _self self)
  (bind _returnvalue (Transformation|GetActorLocation _self))
  ;[0 0 0] Zoom
  (:Pressed
    (Transformation|SetActorLocation _self (Math|Vector|MakeVector (.x _returnvalue) (.y _returnvalue) (- (.z _returnvalue) (Variables|Default|GetZoom))) false false)))

(event Input|MouseEvents|MouseWheelDown
  (params (Key :type Key%20Structure :default "None"))
  (bind _self self)
  (bind _returnvalue (Transformation|GetActorLocation _self))
  ;[0 0 0] Zoom
  (:Pressed
    (Transformation|SetActorLocation _self (Math|Vector|MakeVector (.x _returnvalue) (.y _returnvalue) (+ (.z _returnvalue) (Variables|Default|GetZoom))) false false)))

(fn ConstructionScript)