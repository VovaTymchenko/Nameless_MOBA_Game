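; Player controller for a MOBA-style game, driving a separate camera and champion found at BeginPlay.
; Tick edge-pans the camera using hardcoded 1080p bounds, while the mouse wheel changes its height.
; Clicks trace under the cursor to toggle a print-only shop, target enemies or set destinations.
; Tick moves the champion through its AI controller, firing homing projectiles at in-range targets on an attack-speed cooldown.
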(event Custom|Chase
  (params (WalkTarget :type Actor%20Object%20Reference))
  (bind _pawnchampion (Variables|Default|GetPawnChampion))
  (AI|Navigation|MovetoActor (AI|GetAIController _pawnchampion) WalkTarget (Variables|/Game/Champion/BP_Champion.BP_Champion_C|GetAttackRange _pawnchampion) false true false 0))

(event Custom|Walk
  (params (WalkTarget :type Vector))
  (AI|Navigation|MovetoLocation (AI|GetAIController (Variables|Default|GetPawnChampion)) WalkTarget 1e+01 false true false false 0))

(event EventBeginPlay
  (Variables|Default|SetbShowMouseCursor true)
  ;[0 0 0] Camera
  (bind _returnvalue (Actor|GetActorOfClass "/Game/Game/BP_Camera.BP_Camera_C"))
  (Variables|Default|SetPawnCamera _returnvalue)
  ;[0 0 0] Champion
  (bind _returnvalue_2 (Actor|GetActorOfClass "/Game/Champion/BP_Champion.BP_Champion_C"))
  (Variables|Default|SetPawnChampion _returnvalue_2))

(event EventTick
  (params (DeltaSeconds :type Float%20%28single-precision%29))
  (bind _pawncamera (Variables|Default|GetPawnCamera))
  (bind _pawncamera_2 (Variables|Default|GetPawnCamera))
  (bind _pawncamera_3 (Variables|Default|GetPawnCamera))
  (bind _pawncamera_4 (Variables|Default|GetPawnCamera))
  (bind _pawncamera_5 (Variables|Default|GetPawnCamera))
  (bind _returnvalue (Transformation|GetActorLocation _pawncamera_4))
  (bind _returnvalue_2 (Transformation|GetActorLocation _pawncamera_2))
  (bind _returnvalue_3 (Transformation|GetActorLocation _pawncamera_3))
  (bind _returnvalue_4 (Transformation|GetActorLocation _pawncamera_5))
  (bind _speed (Variables|/Game/Game/BP_Camera.BP_Camera_C|GetSpeed _pawncamera))
  (bind _returnvalue_5 (Class|WidgetLayoutLibrary|GetMousePositiononPlatform))
  (Utilities|FlowControl|Sequence
    (:then_0
      ;[0 0 0] Camera X
      (if (< (.y _returnvalue_5) 1.0)
        (Transformation|SetActorLocation _pawncamera_2 (Math|Vector|MakeVector (+ (.x _returnvalue_2) _speed) (.y _returnvalue_2) (.z _returnvalue_2)) false false)
        (elif (> (.y _returnvalue_5) 1078.0)
          (Transformation|SetActorLocation _pawncamera_3 (Math|Vector|MakeVector (- (.x _returnvalue_3) _speed) (.y _returnvalue_3) (.z _returnvalue_3)) false false))))
    (:then_1
      ;[0 0 0] Camera Y
      (if (< (.x _returnvalue_5) 1.0)
        (Transformation|SetActorLocation _pawncamera_4 (Math|Vector|MakeVector (.x _returnvalue) (- (.y _returnvalue) _speed) (.z _returnvalue)) false false)
        (elif (> (.x _returnvalue_5) 1918.0)
          (Transformation|SetActorLocation _pawncamera_5 (Math|Vector|MakeVector (.x _returnvalue_4) (+ (.y _returnvalue_4) _speed) (.z _returnvalue_4)) false false))))
    (:then_2
      (bind _attackready (CallFunction|Reload DeltaSeconds))
      (Utilities|IsValid (Variables|Default|GetAttackTarget)
        (:Is%20Valid
          (if _attackready
            (bind _withinattackrange (CallFunction|WithinAttackRange))
            (if _withinattackrange
              (CallFunction|Attack)
              (else
                (CallFunction|Chase (Variables|Default|GetAttackTarget))))))
        (:Is%20Not%20Valid
          (if (Variables|Default|GetisWalking)
            (CallFunction|Walk (Variables|Default|GetWalkTarget))))))))

(event Input|ActionEvents|InputActionShop
  (params (Key :type Key%20Structure :default "None"))
  (:Pressed
    (Utilities|FlowControl|FlipFlop
      (:A
        (CallFunction|OpenShop))
      (:B
        (CallFunction|CloseShop)))))

(event Input|ActionEvents|InputActionPrimaryAction
  (params (Key :type Key%20Structure :default "None"))
  (bind (_worldlocation _worlddirection) (Game|Player|ConvertMouseLocationToWorldSpace))
  (:Pressed
    (Class|NavMovementComponent|StopActiveMovement (Variables|/Script/Engine.Character|GetCharacterMovement (Variables|Default|GetPawnChampion)))
    (bind _outhit (Collision|LineTraceByChannel _worldlocation (+ _worldlocation (* _worlddirection 1e+05)) "TraceTypeQuery1" false 0 "Persistent"))
    (Variables|Default|SetAttackTarget 0)
    (if (Actor|ActorHasTag (.hitactor _outhit) "Shop")
      (Utilities|FlowControl|FlipFlop
        (:A
          (CallFunction|OpenShop))
        (:B
          (CallFunction|CloseShop)))
      (else
        (bind (_teamblue _canbeattacked) (Class|BIAnswerTeam|AnswerTeam(Message) (.hitactor _outhit)))
        (if (and _canbeattacked (!= _teamblue (Variables|/Game/Champion/BP_Champion.BP_Champion_C|GetTeamBlue (Variables|Default|GetPawnChampion))))
          (bind _output_get (Variables|Default|SetAttackTarget (.hitactor _outhit)))
          (Variables|Default|SetWalkTarget (Transformation|GetActorLocation _output_get))
          (Variables|Default|SetisWalking true)
          (else
            (Variables|Default|SetWalkTarget (.location _outhit))
            (Variables|Default|SetisWalking true)))))))

(event Input|ActionEvents|InputActionCancelActions
  (params (Key :type Key%20Structure :default "None"))
  (:Pressed
    (Class|NavMovementComponent|StopActiveMovement (Variables|/Script/Engine.Character|GetCharacterMovement (Variables|Default|GetPawnChampion)))
    (Variables|Default|SetAttackTarget 0)
    (Variables|Default|SetisWalking false)))

(event Input|MouseEvents|MouseWheelDown
  (params (Key :type Key%20Structure :default "None"))
  (bind _pawncamera (Variables|Default|GetPawnCamera))
  (bind _returnvalue (Transformation|GetActorLocation _pawncamera))
  ;[0 0 0] Camera Zoom
  (:Pressed
    (Transformation|SetActorLocation _pawncamera (Math|Vector|MakeVector (.x _returnvalue) (.y _returnvalue) (+ (.z _returnvalue) (Variables|/Game/Game/BP_Camera.BP_Camera_C|GetZoom (Variables|Default|GetPawnCamera)))) false false)))

(event Input|MouseEvents|MouseWheelUp
  (params (Key :type Key%20Structure :default "None"))
  (bind _pawncamera (Variables|Default|GetPawnCamera))
  (bind _returnvalue (Transformation|GetActorLocation _pawncamera))
  ;[0 0 0] Camera Zoom
  (:Pressed
    (Transformation|SetActorLocation _pawncamera (Math|Vector|MakeVector (.x _returnvalue) (.y _returnvalue) (- (.z _returnvalue) (Variables|/Game/Game/BP_Camera.BP_Camera_C|GetZoom (Variables|Default|GetPawnCamera)))) false false)))

(fn ConstructionScript)

(fn OpenShop
  (Development|PrintString "open shop")
  (return))

(fn CloseShop
  (Development|PrintString "close shop")
  (return))

(fn Reload
  (params (TimePassed :type Float%20%28double-precision%29))
  (bind _output_get (Variables|Default|SetReloadRate (- (Variables|Default|GetReloadRate) TimePassed)))
  (if (<= _output_get 0.0)
    (Variables|Default|SetReloadRate 0.0))
  (return (<= _output_get 0.0)))

(fn Attack
  (bind _returnvalue (Game|SpawnActorfromClass "/Game/BP_Projectile.BP_Projectile_C" (Math|Transform|MakeTransform (Transformation|GetActorLocation (Variables|Default|GetPawnChampion))) "AlwaysSpawn" 0 0))
  (Variables|/Game/BP_Projectile.BP_Projectile_C|SetHomingTarget _returnvalue (Variables|Default|GetAttackTarget))
  (Variables|Default|SetReloadRate (/ 1.0 (Variables|/Game/Champion/BP_Champion.BP_Champion_C|GetAttackSpeed (Variables|Default|GetPawnChampion)))))

(fn WithinAttackRange
  (bind _pawnchampion (Variables|Default|GetPawnChampion))
  (bind _attacktarget (Variables|Default|GetAttackTarget))
  (bind _actorradius (Class|BIAnswerActorRadius|AnswerActorRadius(Message) _attacktarget))
  (return (< (Math|Vector|Distance(Vector) (Transformation|GetActorLocation _pawnchampion) (Transformation|GetActorLocation _attacktarget)) (+ _actorradius (Variables|/Game/Champion/BP_Champion.BP_Champion_C|GetAttackRange _pawnchampion)))))