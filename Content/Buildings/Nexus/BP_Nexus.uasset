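; BP_Nexus is a team-owned Nexus building whose destruction is meant to end the game.
; It answers team, attackability and radius queries, and applies damage through CalculateDamage with physical and magic resistances, or clamped healing.
; Health changes feed its widget health bar.
; On death it shows WB_GameEnd, but the pause is immediately undone and the main menu step is only a debug print.
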(event EventBeginPlay
  (bind _aswb_tower_health_bar (Utilities|Casting|CastToWB_Tower_HealthBar (UserInterface|GetUserWidgetObject (Variables|Default|GetHealthBarWidget))))
  (Variables|Default|SetHealthBar _aswb_tower_health_bar)
  (Variables|/Game/Buildings/Tower/UI/WB_Tower_HealthBar.WB_Tower_HealthBar_C|SetMaxHealth _aswb_tower_health_bar (Variables|Default|GetHealth))
  (Variables|/Game/Buildings/Tower/UI/WB_Tower_HealthBar.WB_Tower_HealthBar_C|SetHealth _aswb_tower_health_bar (Variables|Default|GetHealth)))

(fn ConstructionScript
  (|CallParentFunction))

(fn AnswerTeam
  (return (Variables|Default|GetTeamBlue) (Variables|Default|GetCanBeAttacked)))

(fn AnswerActorRadius
  (return (Variables|Default|GetRadius)))

(fn ReceiveDamage
  (params (TrueDamage :type Float%20%28double-precision%29) (PhysDamage :type Float%20%28double-precision%29) (MagicDamage :type Float%20%28double-precision%29) (Attacker :type Actor%20Object%20Reference))
  (bind (_killed _healthleft) (CallFunction|CalculateDamage (Variables|Default|GetHealth) TrueDamage PhysDamage (Variables|Default|GetPhysResist) MagicDamage (Variables|Default|GetMagicResist)))
  (Variables|Default|SetHealth _healthleft)
  (if _killed
    ;[1 0 0] pls just do something with this
    (Development|PrintString "END GAMMEEE!!!!")
    (Game|SetGamePaused true)
    (bind _returnvalue (UserInterface|CreateWidget "/Game/UI/WB_GameEnd.WB_GameEnd_C"))
    (UserInterface|Viewport|AddtoViewport _returnvalue 0)
    (Game|SetGamePaused false)
    (Development|PrintString "open main menu")
    (return true)
    (else
      (Variables|/Game/Buildings/Tower/UI/WB_Tower_HealthBar.WB_Tower_HealthBar_C|SetHealth (Variables|Default|GetHealthBar) (Variables|Default|Gethealth))
      (return false))))

(fn ReceiveHealing
  (params (HealAmount :type Float%20%28double-precision%29) (Healer :type Actor%20Object%20Reference))
  (Variables|Default|SetHealth (Math|Float|Clamp(Float) (+ HealAmount (Variables|Default|GetHealth)) 0.0 (Variables|Default|GetMaxHealth)))
  (Variables|/Game/Buildings/Tower/UI/WB_Tower_HealthBar.WB_Tower_HealthBar_C|SetHealth (Variables|Default|GetHealthBar) (Variables|Default|Gethealth))
  (return (== (Variables|Default|GetHealth) (Variables|Default|GetMaxHealth))))