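; BP_Inhibitor is a Blue team inhibitor building that spawns minions and can be destroyed.
; From BeginPlay, a looping Delay spawns a BP_unMinion running BT_unMinion every 30 seconds at a hardcoded world location, independent of the building's position.
; Damage events subtract from Health, print the remaining value and destroy the actor at zero or below, which also ends spawning.
; AnswerTeam always reports TeamBlue.
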(event EventDamage
  (params (Damage :type Float%20%28double-precision%29) (Attacker :type Actor%20Object%20Reference))
  (bind _output_get (Variables|Default|SetHealth (- (Variables|Default|GetHealth) Damage)))
  (Development|PrintString (Utilities|String|ToString(Float) _output_get))
  (if (<= _output_get 0.0)
    (Actor|DestroyActor)))

(event EventBeginPlay
  (AI|SpawnAIFromClass "/Game/unMinion/BP_unMinion.BP_unMinion_C" "/Game/unMinion/BT_unMinion.BT_unMinion" (Math|Vector|MakeVector 0.0 6e+03 1e+02) "0, 0, 0" true 0 :!label _label)
  (Utilities|FlowControl|Delay 3e+01)
  (goto _label))

(fn ConstructionScript
  (|CallParentFunction))

(fn AnswerTeam
  (return (Variables|Default|GetTeamBlue)))