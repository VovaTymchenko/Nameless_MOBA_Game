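; BP_Nexus is a team's Nexus building that answers queries for its team and radius and reports itself as attackable.
; ReceiveDamage ignores all damage inputs and simply returns false.
; A disconnected end-game chain would destroy the actor, pause the game and show the WB_GameEnd widget, then unpause with a main-menu debug print, but it never runs.
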(fn ConstructionScript
  (|CallParentFunction))

(fn AnswerTeam
  (return (Variables|Default|GetTeamBlue) true))

(fn AnswerActorRadius
  (return (Variables|Default|GetRadius)))

(fn ReceiveDamage
  (params (TrueDamage :type Float%20%28double-precision%29) (PhysDamage :type Float%20%28double-precision%29) (MagicDamage :type Float%20%28double-precision%29) (Attacker :type Actor%20Object%20Reference))
  (return false))