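; BP_Inhibitor is a team-owned, attackable building that spawns AI minions and can be destroyed by damage.
; From BeginPlay it loops endlessly, spawning a BP_Minion running BT_Minion at a hardcoded world location, then waiting a fixed delay.
; Query functions report its team, attackability and radius.
; Receive Damage resolves true, physical and magic damage against resistances, prints remaining health, and destroys the actor on a kill, returning whether it died.
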(event EventBeginPlay
  (AI|SpawnAIFromClass "/Game/Minion/BP_Minion.BP_Minion_C" "/Game/Minion/BT_Minion.BT_Minion" (Math|Vector|MakeVector 6e+03 2e+03 1e+02) "0, 0, 0" true 0 :!label _label)
  (Utilities|FlowControl|Delay 2e+01)
  (goto _label))

(fn ConstructionScript
  (|CallParentFunction))

(fn AnswerTeam
  (return (Variables|Default|GetTeamBlue) true))

(fn AnswerActorRadius
  (return (Variables|Default|GetRadius)))

(fn ReceiveDamage
  (params (TrueDamage :type Float%20%28double-precision%29) (PhysDamage :type Float%20%28double-precision%29) (MagicDamage :type Float%20%28double-precision%29) (Attacker :type Actor%20Object%20Reference))
  (bind (_killed _healthleft) (CallFunction|CalculateDamage (Variables|Default|GetHealth) TrueDamage PhysDamage (Variables|Default|GetPhysResist) MagicDamage (Variables|Default|GetMagicResist)))
  (bind _output_get (Variables|Default|SetHealth _healthleft))
  (Development|PrintString (Utilities|String|ToString(Float) _output_get))
  (if _killed
    (Actor|DestroyActor)
    (return true)
    (else
      (return false))))