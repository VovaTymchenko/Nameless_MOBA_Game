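; BP_Tower is a team-owned tower building with health, resistances, a health bar widget and a gold bounty.
; A sphere sized to AttackRange adds attackable enemy-team actors to TargetList on overlap, though no firing or target removal appears here.
; Team and radius queries answer other actors, while ReceiveDamage applies typed damage, updates the bar, and on death disables targeting and only prints the bounty.
; Healing clamps Health without refreshing the bar.
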(event OnComponentBeginOverlap(SphereCollider)
  (params (OverlappedComponent :type Primitive%20Component%20Object%20Reference) (OtherActor :type Actor%20Object%20Reference) (OtherComp :type Primitive%20Component%20Object%20Reference) (OtherBodyIndex :type Integer) (bFromSweep :type Boolean) (SweepResult :type Hit%20Result%20Structure%20%28by%20ref%29))
  ;[0 0 0] Add target to the list on collision
  (bind (_teamblue _canbeattacked) (Class|BIAnswerTeam|AnswerTeam(Message) OtherActor))
  (if (and _canbeattacked (!= _teamblue (Variables|Default|GetTeamBlue)))
    (Utilities|Array|Add (Variables|V_Tech|GetTargetList) OtherActor)))

(event EventHealing
  (params (HealAmount :type Float%20%28double-precision%29) (Healer :type Actor%20Object%20Reference))
  (Variables|Default|SetHealth (Math|Float|Clamp(Float) (+ HealAmount (Variables|Default|GetHealth)) 0.0 (Variables|Default|GetMaxHealth))))

(event EventBeginPlay
  (bind _aswb_tower_health_bar (Utilities|Casting|CastToWB_Tower_HealthBar (UserInterface|GetUserWidgetObject (Variables|Default|GetHealthBarWidget))))
  (Variables|V_Tech|SetHealthBar _aswb_tower_health_bar)
  (Variables|/Game/Buildings/Tower/UI/WB_Tower_HealthBar.WB_Tower_HealthBar_C|SetMaxHealth _aswb_tower_health_bar (Variables|Default|GetHealth))
  (Variables|/Game/Buildings/Tower/UI/WB_Tower_HealthBar.WB_Tower_HealthBar_C|SetHealth _aswb_tower_health_bar (Variables|Default|GetHealth)))

(fn ConstructionScript
  (|CallParentFunction)
  (Components|Sphere|SetSphereRadius (Variables|Default|GetSphereCollider) (Variables|V_Stats|GetAttackRange) true))

(fn ReceiveDamage
  (params (TrueDamage :type Float%20%28double-precision%29) (PhysDamage :type Float%20%28double-precision%29) (MagicDamage :type Float%20%28double-precision%29) (Attacker :type Actor%20Object%20Reference))
  (bind (_killed _healthleft) (CallFunction|CalculateDamage (Variables|Default|GetHealth) TrueDamage PhysDamage (Variables|Default|GetPhysResist) MagicDamage (Variables|Default|GetMagicResist)))
  (bind _output_get (Variables|Default|SetHealth _healthleft))
  ;[1 0 0] HB-reomve latr
  (Development|PrintString (Utilities|String|ToString(Float) _output_get))
  (if _killed
    (Variables|Default|SetCanBeAttacked false)
    ;[1 0 0] GIVE GOLD
    (Development|PrintString (Utilities|String|Append (Utilities|GetDisplayName Attacker) "gets " (Utilities|String|ToString(Integer) (Variables|Default|GetBounty)) " gold for destroying a building" (Utilities|GetDisplayName self)))
    (return true)
    (else
      (Variables|/Game/Buildings/Tower/UI/WB_Tower_HealthBar.WB_Tower_HealthBar_C|SetHealth (Variables|V_Tech|GetHealthBar) (Variables|Default|Gethealth))
      (return false))))

(fn AnswerTeam
  (return (Variables|Default|GetTeamBlue) (Variables|Default|GetCanBeAttacked)))

(fn AnswerActorRadius
  (return (Variables|Default|GetRadius)))