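; Minion projectile actor that homes in on a single HomingTarget and damages it on contact.
; Shortly after BeginPlay, it points ProjectileMovement's homing component at the target's root component.
; Overlapping that target sends a fixed damage message naming the projectile itself as attacker, then destroys the projectile; other actors are ignored.
; Tick destroys the projectile whenever the target is no longer valid.
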(event Collision|EventActorBeginOverlap
  (params (OtherActor :type Actor%20Object%20Reference))
  (if (== OtherActor (Variables|Default|GetHomingTarget))
    (Class|BIReceiveDamage|ReceiveDamage(Message) OtherActor 2e+01 self)
    (Actor|DestroyActor)))

(event EventBeginPlay
  (Utilities|FlowControl|Delay 0.1)
  (Variables|/Script/Engine.ProjectileMovementComponent|SetHomingTargetComponent (Variables|Default|GetProjectileMovement) (Variables|/Script/Engine.Actor|GetRootComponent (Variables|Default|GetHomingTarget))))

(event EventTick
  (params (DeltaSeconds :type Float%20%28single-precision%29))
  (Utilities|IsValid (Variables|Default|GetHomingTarget)
    (:Is%20Not%20Valid
      (Actor|DestroyActor))))

(fn ConstructionScript)