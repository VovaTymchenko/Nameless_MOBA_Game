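; Team-based minion that tracks attackable enemies and picks checkpoints as walk targets, with a health bar widget.
; A range-sized sphere adds overlapping enemies to a target list; an enemy checkpoint still unvisited becomes the walk target.
; Construction gathers all checkpoints and selects the nearest, removing each chosen one from the remaining list.
; It answers team and radius queries, and applies true, physical and magic damage against resistances, destroying itself on death.
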(event OnComponentBeginOverlap(Sphere)
  (params (OverlappedComponent :type Primitive%20Component%20Object%20Reference) (OtherActor :type Actor%20Object%20Reference) (OtherComp :type Primitive%20Component%20Object%20Reference) (OtherBodyIndex :type Integer) (bFromSweep :type Boolean) (SweepResult :type Hit%20Result%20Structure%20%28by%20ref%29))
  ;[0 0 0] Add target to the list on collision
  (bind (_teamblue _canbeattacked) (Class|BIAnswerTeam|AnswerTeam(Message) OtherActor))
  (if (and _canbeattacked (!= _teamblue (Variables|Default|GetTeamBlue)))
    (Utilities|Array|Add (Variables|Default|GetTargetList) OtherActor)
    (bind _asbp_checkpoint (Utilities|Casting|CastToBP_Checkpoint OtherActor))
    (if (Utilities|Array|ContainsItem (Variables|Default|GetCheckpoints) _asbp_checkpoint)
      (CallFunction|SetNextCheckpoint true _asbp_checkpoint))))

(event EventBeginPlay
  (bind _aswb_health_bar (Utilities|Casting|CastToWB_HealthBar (UserInterface|GetUserWidgetObject (Variables|Default|GetWidget))))
  (Variables|Default|SetHealthBar _aswb_health_bar)
  (Variables|/Game/UI/WB_HealthBar.WB_HealthBar_C|SetMaxHealth _aswb_health_bar (Variables|Default|GetHealth))
  (Variables|/Game/UI/WB_HealthBar.WB_HealthBar_C|SetHealth _aswb_health_bar (Variables|Default|GetHealth)))

(fn ConstructionScript
  (Components|Sphere|SetSphereRadius (Variables|Default|GetSphere) (Variables|Default|GetTargetRange) true)
  (bind _outactors (Actor|GetAllActorsOfClass "/Game/Minion/BP_Checkpoint.BP_Checkpoint_C"))
  (Variables|Default|SetCheckpoints _outactors)
  (CallFunction|SetNextCheckpoint false)
  (Variables|Default|SetOldCheckpoint (Variables|Default|GetWalkTarget)))

(fn SetNextCheckpoint
  (params (Collided :type Boolean) (New%20Checkpoint :type Actor%20Object%20Reference))
  (bind _checkpoints (Variables|Default|GetCheckpoints))
  (Variables|Default|SetOldCheckpoint (Variables|Default|GetWalkTarget))
  (if Collided
    (bind _output_get (Variables|Default|SetWalkTarget New%20Checkpoint))
    (Utilities|Array|RemoveItem (Variables|Default|GetCheckpoints) _output_get)
    (return)
    (else
      (bind _output_get_2 (Variables|Default|SetWalkTarget (.ReturnValue (Actor|FindNearestActor (Transformation|GetActorLocation self) _checkpoints))))
      (Utilities|Array|RemoveItem _checkpoints _output_get_2)
      (return))))

(fn AnswerActorRadius
  (return (Variables|Default|GetRadius)))

(fn AnswerTeam
  (return (Variables|Default|GetTeamBlue) true))

(fn ReceiveDamage
  (params (TrueDamage :type Float%20%28double-precision%29) (PhysDamage :type Float%20%28double-precision%29) (MagicDamage :type Float%20%28double-precision%29) (Attacker :type Actor%20Object%20Reference))
  (bind (_killed _healthleft) (CallFunction|CalculateDamage (Variables|Default|GetHealth) TrueDamage PhysDamage (Variables|Default|GetPhysResist) MagicDamage (Variables|Default|GetMagicResist)))
  (bind _output_get (Variables|Default|SetHealth _healthleft))
  (Development|PrintString (Utilities|String|ToString(Float) _output_get))
  (if _killed
    (Actor|DestroyActor)
    (return true)
    (else
      (Variables|/Game/UI/WB_HealthBar.WB_HealthBar_C|SetHealth (Variables|Default|GetHealthBar) (Variables|Default|GetHealth))
      (return false))))