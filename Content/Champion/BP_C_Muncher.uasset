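; Muncher champion Blueprint with four placeholder abilities that call their parent versions and print their q, w, e or r key letter.
; Damage runs health and resistances through CalculateDamage, destroying the actor on death and returning whether it was killed.
; Healing and mana gain clamp to their maximums and report when full.
; LoseMana ignores its decrease amount and clamps negated Mana, which empties the pool for any non-negative value.
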(fn ConstructionScript
  (|CallParentFunction))

(fn Ability1
  (|CallParentFunction)
  (Development|PrintString "q"))

(fn Ability2
  (|CallParentFunction)
  (Development|PrintString "w"))

(fn Ability3
  (|CallParentFunction)
  (Development|PrintString "e"))

(fn Ability4
  (|CallParentFunction)
  (Development|PrintString "r"))

(fn ReceiveDamage
  (params (TrueDamage :type Float%20%28double-precision%29) (PhysDamage :type Float%20%28double-precision%29) (MagicDamage :type Float%20%28double-precision%29) (Attacker :type Actor%20Object%20Reference))
  (bind (_killed _healthleft) (CallFunction|CalculateDamage (Variables|Default|GetHealth) TrueDamage PhysDamage (Variables|Default|GetPhysResist) MagicDamage (Variables|Default|GetMagicResist)))
  (Variables|Default|SetHealth _healthleft)
  (if _killed
    (Actor|DestroyActor)
    (return true)
    (else
      (return false))))

(fn ReceiveHealing
  (params (HealAmount :type Float%20%28double-precision%29) (Healer :type Actor%20Object%20Reference))
  (Variables|Default|SetHealth (Math|Float|Clamp(Float) (+ HealAmount (Variables|Default|GetHealth)) 0.0 (Variables|Default|GetMaxHealth)))
  (return (== (Variables|Default|GetHealth) (Variables|Default|GetMaxHealth))))

(fn GainMana
  (params (ManaIncrease :type Float%20%28double-precision%29) (Initiator :type Actor%20Object%20Reference))
  (Variables|Default|SetMana (Math|Float|Clamp(Float) (+ ManaIncrease (Variables|Default|GetMana)) 0.0 (Variables|Default|GetMaxMana)))
  (return (== (Variables|Default|GetMana) (Variables|Default|GetMaxMana))))

(fn LoseMana
  (params (ManaDecrease :type Float%20%28double-precision%29) (Initiator :type Actor%20Object%20Reference))
  (Variables|Default|SetMana (Math|Float|Clamp(Float) (- 0.0 (Variables|Default|GetMana)) 0.0 (Variables|Default|GetMaxMana)))
  (return (== (Variables|Default|GetMana) 0.0)))