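; BP_Champion is a champion that takes damage and can be queried for its team and size.
; The Damage event subtracts from Health, prints the new value and destroys the actor once Health reaches zero or below.
; AnswerActorRadius returns the stored Radius, while AnswerTeam returns the TeamBlue value and always reports the champion as attackable.
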(event EventDamage
  (params (Damage :type Float%20%28double-precision%29) (Attacker :type Actor%20Object%20Reference))
  (bind _output_get (Variables|Default|SetHealth (- (Variables|Default|GetHealth) Damage)))
  (Development|PrintString (Utilities|String|ToString(Float) _output_get))
  (if (<= _output_get 0.0)
    (Actor|DestroyActor)))

(fn ConstructionScript)

(fn AnswerActorRadius
  (return (Variables|Default|GetRadius)))

(fn AnswerTeam
  (return (Variables|Default|GetTeamBlue) true))