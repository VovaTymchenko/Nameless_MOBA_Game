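; BP_unMinion is a blue-team minion with health that can be damaged and destroyed.
; On BeginPlay it stores the location of a BP_Building as WalkTarget, and its sphere overlap adds actors not answering TeamBlue to TargetList.
; Damage events reduce Health, destroying it at zero and printing the attacker's name.
; Movement, attacking and health bar updates are absent from these graphs.
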(event OnComponentBeginOverlap(Sphere)
  (params (OverlappedComponent :type Primitive%20Component%20Object%20Reference) (OtherActor :type Actor%20Object%20Reference) (OtherComp :type Primitive%20Component%20Object%20Reference) (OtherBodyIndex :type Integer) (bFromSweep :type Boolean) (SweepResult :type Hit%20Result%20Structure%20%28by%20ref%29))
  ;[0 0 0] Add target to the list on collision
  (bind _teamblue (Class|BIAnswerTeam|AnswerTeam(Message) OtherActor))
  (if (!= _teamblue (Variables|Default|GetTeamBlue))
    (Utilities|Array|Add (Variables|Default|GetTargetList) OtherActor)
    (else
      (Development|PrintString "No Hello!!!"))))

(event EventBeginPlay
  (bind _returnvalue (Actor|GetActorOfClass "/Game/Buildings/BP_Building.BP_Building_C"))
  (Variables|Default|SetWalkTarget (Transformation|GetActorLocation _returnvalue)))

(event EventDamage
  (params (Damage :type Float%20%28double-precision%29) (Attacker :type Actor%20Object%20Reference))
  (bind _output_get (Variables|Default|SetHealth (- (Variables|Default|GetHealth) Damage)))
  (if (<= _output_get 0.0)
    (Actor|DestroyActor)
    (Development|PrintString (Utilities|GetDisplayName Attacker))))

(event EventTick
  (params (DeltaSeconds :type Float%20%28single-precision%29))
  ;[1 0 0] healthbar widget - cant bind (hard to reference instance)
)

(fn ConstructionScript)

(fn AnswerTeam
  (return (Variables|Default|GetTeamBlue)))