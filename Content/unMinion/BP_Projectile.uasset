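; BP_Projectile is a homing projectile that damages its assigned target on contact.
; Shortly after BeginPlay it asks HomingTarget, through a message call, for a component and sets that as the ProjectileMovement homing target.
; When it overlaps that target, and only that target, it sends a fixed-damage message naming itself as attacker, then destroys itself.
; Tick is an empty stub, so target validity is never rechecked.
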(event Collision|EventActorBeginOverlap
  (params (OtherActor :type Actor%20Object%20Reference))
  (if (== OtherActor (Variables|Default|GetHomingTarget))
    (Class|BIReceiveDamage|ReceiveDamage(Message) OtherActor 2e+01 self)
    (Actor|DestroyActor)))

(event EventBeginPlay
  (Utilities|FlowControl|Delay 0.1)
  (bind _targetcomponent (Class|BIAnswerHomingProjectileTarget|AnswerHomingProjectileTargetComponent(Message) (Variables|Default|GetHomingTarget)))
  (Variables|/Script/Engine.ProjectileMovementComponent|SetHomingTargetComponent (Variables|Default|GetProjectileMovement) _targetcomponent))

(event EventTick
  (params (DeltaSeconds :type Float%20%28single-precision%29))
  ;[1 1 1] check the target is still valid
)

(fn ConstructionScript)